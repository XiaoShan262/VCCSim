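; Cinematic car rig pawn that drives a car along a spline path by traveled distance, updating on Tick, in the construction script and via a looping editor timer.
; It steers toward the spline ahead and can line-trace actor and wheels to the ground, deriving chassis roll, pitch and position from the wheels.
; Distance-driven wheel spin, suspension-lagged body motion and Perlin noise vibration add realism, with drift, camber and brake lock controls.
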(event EventEditorTick
  (if (Variables|CarSetup|GetTrackPath)
    (if (Variables|CarSetup|GetEditorUpdate)
      (Utilities|FlowControl|Sequence
        (:then_0
          (CallFunction|SetTraceIgnores)
          ;[0 0 0] Path
          (CallFunction|CalculateDistance)
          (CallFunction|FollowthePathandSteer)
          ;[0 0 0] Reset and Initialize
          (CallFunction|ActorGroundTrace)
          (CallFunction|InitialState)
          (if (Variables|CarSetup|GetTraceGround)
            ;[0 0 0] Tracing Ground
            (for _index (range 0 1)
              (CallFunction|WheelsGroundTrace)
              (CallFunction|ChassisRollandPitch)
              (CallFunction|ChassisRelocation)
              (CallFunction|BodyDelay true))
            (else
              ;[0 0 0] Final Steps
              (CallFunction|BodyDelay false)))
          (CallFunction|WheelsDrive)
          (CallFunction|Vibrations)
          (CallFunction|CalipersPlacement)
          (CallFunction|CalculateSpeed))
        (:then_1
          (CallFunction|AutoMove (stale EventTick DeltaSeconds)))))))

(event EventTick
  (params (DeltaSeconds :type Float%20%28single-precision%29))
  (Variables|CarSetup|SetTickFPS (/ 1.0 DeltaSeconds))
  (if (Variables|CarSetup|GetTrackPath)
    (Utilities|FlowControl|Sequence
      (:then_0
        (CallFunction|SetTraceIgnores)
        ;[0 0 0] Path
        (CallFunction|CalculateDistance)
        (CallFunction|FollowthePathandSteer)
        ;[0 0 0] Reset and Initialize
        (CallFunction|ActorGroundTrace)
        (CallFunction|InitialState)
        (if (Variables|CarSetup|GetTraceGround)
          ;[0 0 0] Tracing Ground
          (for _index (range 0 1)
            (CallFunction|WheelsGroundTrace)
            (CallFunction|ChassisRollandPitch)
            (CallFunction|ChassisRelocation)
            (CallFunction|BodyDelay true))
          (else
            ;[0 0 0] Final Steps
            (CallFunction|BodyDelay false)))
        (CallFunction|WheelsDrive)
        (CallFunction|Vibrations)
        (CallFunction|CalipersPlacement)
        (CallFunction|CalculateSpeed))
      (:then_1
        (CallFunction|AutoMove DeltaSeconds)))))

(fn ConstructionScript
  (CallFunction|StartEditorTick)
  (CallFunction|SetTraceIgnores)
  (CallFunction|CarMeshSetup)
  ;[0 0 0] Path
  (CallFunction|CalculateDistance)
  (CallFunction|FollowthePathandSteer)
  ;[0 0 0] Reset and Initialize
  (CallFunction|ActorGroundTrace)
  (CallFunction|InitialState)
  (if (Variables|CarSetup|GetTraceGround)
    ;[0 0 0] Tracing Ground
    (for _index (range 0 1)
      (CallFunction|WheelsGroundTrace)
      (CallFunction|ChassisRollandPitch)
      (CallFunction|ChassisRelocation)))
  ;[0 0 0] Final Steps
  (CallFunction|BodyDelay false)
  (CallFunction|WheelsDrive)
  (CallFunction|Vibrations)
  (CallFunction|CalipersPlacement)
  (CallFunction|CalculateSpeed))

(fn InitialState
  (bind _rearcamber (Variables|Suspension|GetRearCamber))
  (bind _frontcamber (Variables|Suspension|GetFrontCamber))
  (bind _frontaxleoffset (Variables|CarSetup|GetFrontAxleOffset))
  (bind _rearaxleoffset (Variables|CarSetup|GetRearAxleOffset))
  (bind _frontwheelssideoffset (Variables|CarSetup|GetFrontWheelsSideOffset))
  (bind _rearwheelssideoffset (Variables|CarSetup|GetRearWheelsSideOffset))
  (bind _drift (Variables|Driving|GetDrift))
  (bind _steering (Variables|Driving|GetSteering))
  (bind _overallvibrationmultiplier (Variables|Vibrations|GetOverallVibrationMultiplier))
  (bind _returnvalue (Math|Float|Clamp(Float) _steering -45.0 45.0))
  (bind _returnvalue_2 (Math|Float|Clamp(Float) _drift -4e+01 4e+01))
  (bind _returnvalue_3 (Math|Float|Clamp(Float) _frontcamber 0.0 1e+01))
  (bind _returnvalue_4 (Math|Float|Clamp(Float) _rearcamber 0.0 1e+01))
  (bind _returnvalue_5 (* _rearaxleoffset -1.0))
  (bind _returnvalue_6 (* _returnvalue_4 -1.0))
  (bind _returnvalue_7 (* -1.0 _returnvalue_3))
  (bind _returnvalue_8 (* _returnvalue_2 _overallvibrationmultiplier))
  (bind _returnvalue_9 (Utilities|PerlinNoise 0.0 0.5 0.1 _returnvalue_8))
  (bind _returnvalue_10 (+ _returnvalue_2 _returnvalue_9))
  (bind _returnvalue_11 (* _returnvalue_10 -1.0))
  (bind _returnvalue_12 (+ _returnvalue _returnvalue_11))
  ;[1 0 1] Reset Chassis to the Initial Transform
  (Transformation|SetRelativeLocationAndRotation (Variables|Default|GetChassis) (Math|Vector|MakeVector 0.0 0.0 (.SphereRadius (Collision|GetComponentBounds (Variables|Default|GetWheel%20FR)))) (Math|Rotator|MakeRotator (+ (Variables|Hidden|GetChassisRoll) (* (Math|Float|MapRangeClamped (Variables|Suspension|GetSuspensionStiffness) 0.0 1e+01 2.0 0.3) (+ (* _returnvalue -0.1) (* _returnvalue_10 -0.1)))) (Variables|Hidden|GetChassisPitch) _returnvalue_10) false false)
  ;[0 1 1] Reset Wheels to the Initial Transform
  (Transformation|SetRelativeLocationAndRotation (Variables|Default|GetWheel%20FR) (Math|Vector|MakeVector _frontaxleoffset _frontwheelssideoffset 0.0) (Math|Rotator|MakeRotator _returnvalue_7 0.0 _returnvalue_12) false false)
  (Transformation|SetRelativeLocationAndRotation (Variables|Default|GetWheel%20FL) (Math|Vector|MakeVector _frontaxleoffset (* _frontwheelssideoffset -1.0) 0.0) (Math|Rotator|MakeRotator _returnvalue_7 0.0 (+ _returnvalue_12 1.8e+02)) false false)
  (Transformation|SetRelativeLocationAndRotation (Variables|Default|GetWheel%20RR) (Math|Vector|MakeVector _returnvalue_5 _rearwheelssideoffset 0.0) (Math|Rotator|MakeRotator _returnvalue_6 0.0 0.0) false false)
  (Transformation|SetRelativeLocationAndRotation (Variables|Default|GetWheel%20RL) (Math|Vector|MakeVector _returnvalue_5 (* _rearwheelssideoffset -1.0) 0.0) (Math|Rotator|MakeRotator _returnvalue_6 0.0 1.8e+02) false false))

(fn WheelsDrive
  (bind _wheel_fl (Variables|Default|GetWheel%20FL))
  (bind _wheel_rl (Variables|Default|GetWheel%20RL))
  (bind _wheel_rr (Variables|Default|GetWheel%20RR))
  (bind _wheel_fr (Variables|Default|GetWheel%20FR))
  ;[0 1 1] Wheels Rotation Based on Traveled Distance
  (if (Variables|Driving|GetRearBreaksLock)
    (if (not (Variables|Driving|GetFrontBreaksLock))
      (Transformation|AddLocalRotation _wheel_fl (Math|Rotator|MakeRotator 0.0 (* (Utilities|CalculateWheelRotation _wheel_fl 1.2e+02) 1.0) 0.0) false false :!label _label)
      (Transformation|AddLocalRotation _wheel_fr (Math|Rotator|MakeRotator 0.0 (* (Utilities|CalculateWheelRotation _wheel_fr -8e+01) -1.0) 0.0) false false))
    (else
      (Transformation|AddLocalRotation _wheel_rl (Math|Rotator|MakeRotator 0.0 (* (Utilities|CalculateWheelRotation _wheel_rl -1.2e+02) 1.0) 0.0) false false)
      (Transformation|AddLocalRotation _wheel_rr (Math|Rotator|MakeRotator 0.0 (* (Utilities|CalculateWheelRotation _wheel_rr 0.0) -1.0) 0.0) false false)
      (if (not (Variables|Driving|GetFrontBreaksLock))
        (goto _label)))))

(fn WheelsGroundTrace
  (bind _chassis (Variables|Default|GetChassis))
  (bind _returnvalue (Math|Vector|GetUpVector _chassis))
  ;[0 1 1] All Wheels Ground Trace
  (for _array_element (Utilities|Array|MakeArray (Variables|Default|GetWheel%20FL) (Variables|Default|GetWheel%20FR) (Variables|Default|GetWheel%20RL) (Variables|Default|GetWheel%20RR))
    (bind _outhit (Collision|LineTraceByChannel (+ (Transformation|GetWorldLocation _array_element) (* _returnvalue 1e+02)) (+ (Transformation|GetWorldLocation _array_element) (* _returnvalue -1e+04)) "TraceTypeQuery1" true (Variables|Hidden|GetActorsToIgnore) (Variables|CarSetup|GetTraceDebug)))
    (if (.bblockinghit _outhit)
      (Transformation|SetWorldLocation _array_element (+ (.impactpoint _outhit) (* _returnvalue (* (.z (.max (StaticMesh|GetBoundingBox (Variables|/Script/Engine.StaticMeshComponent|GetStaticMesh _array_element)))) 0.95))) false false)))
  (return))

(fn FollowthePathandSteer
  (bind _returnvalue (Transformation|GetActorRotation))
  (bind _returnvalue_2 (Transformation|GetActorRotation))
  (bind _path (Variables|Driving|GetPath))
  (bind _coursedistance (Variables|Hidden|GetCourseDistance))
  (bind _coursedistance_2 (Variables|Hidden|GetCourseDistance))
  (bind _path_2 (Variables|Driving|GetPath))
  (bind _spline (Variables|/RatSim/CinematicCarRig/Blueprints/BP_Path.BP_Path_C|GetSpline _path_2))
  (bind _spline_2 (Variables|/RatSim/CinematicCarRig/Blueprints/BP_Path.BP_Path_C|GetSpline _path))
  (if (Variables|CarSetup|GetTraceGround)
    ;[1 0 0] Following the Path and Steering
    (Utilities|IsValid _path_2
      (:Is%20Valid
        (Transformation|SetActorLocationAndRotation (Spline|GetLocationatDistanceAlongSpline _spline _coursedistance_2 "World") (Math|Rotator|MakeRotator 0.0 0.0 (.yaw (Math|Interpolation|RInterpTo _returnvalue (Spline|GetRotationatDistanceAlongSpline _spline _coursedistance_2 "World") (/ 1.0 (Variables|CarSetup|GetTickFPS)) 8.0))))
        (Variables|Driving|SetSteering (Math|Float|Clamp(Float) (Math|Interpolation|FInterpTo (Variables|Driving|GetSteering) (.yaw (Math|Rotator|Delta(Rotator) (Spline|GetRotationatDistanceAlongSpline _spline (+ _coursedistance_2 (Variables|CarSetup|GetFrontAxleOffset)) "World") _returnvalue)) (/ 1.0 (Variables|CarSetup|GetTickFPS)) 3.0) -45.0 45.0))))
    (else
      (Utilities|IsValid _path
        (:Is%20Valid
          (Transformation|SetActorLocationAndRotation (Spline|GetLocationatDistanceAlongSpline _spline_2 _coursedistance "World") (Math|Interpolation|RInterpTo _returnvalue_2 (Spline|GetRotationatDistanceAlongSpline _spline_2 _coursedistance "World") (/ 1.0 (Variables|CarSetup|GetTickFPS)) 8.0))
          (Variables|Driving|SetSteering (Math|Float|Clamp(Float) (Math|Interpolation|FInterpTo (Variables|Driving|GetSteering) (.yaw (Math|Rotator|Delta(Rotator) (Spline|GetRotationatDistanceAlongSpline _spline_2 (+ _coursedistance (Variables|CarSetup|GetFrontAxleOffset)) "World") _returnvalue_2)) (/ 1.0 (Variables|CarSetup|GetTickFPS)) 3.0) -45.0 45.0)))))))

(fn CalipersPlacement
  ;[1 1 0] Relocate Calipers to the Wheels
  (for (_array_element _array_index) (Utilities|Array|MakeArray (Variables|Default|GetCaliper%20RR) (Variables|Default|GetCaliper%20RL) (Variables|Default|GetCaliper%20FR) (Variables|Default|GetCaliper%20FL))
    (Transformation|SetWorldLocation _array_element (Transformation|GetWorldLocation (Utilities|Array|Get(acopy) (Utilities|Array|MakeArray (Variables|Default|GetWheel%20RR) (Variables|Default|GetWheel%20RL) (Variables|Default|GetWheel%20FR) (Variables|Default|GetWheel%20FL)) _array_index)) false false)))

(fn CalculateSpeed
  ;[1 0 0] Calculate Speed by Comparing the Last Distance to Current Distance
  (Variables|ReadOnly|SetSpeed%20%28Km/h%29 (Math|Float|Truncate (* (/ (- (Variables|Hidden|GetCourseDistance) (Variables|Hidden|GetLastCourseDistance)) (/ 1.0 (Variables|CarSetup|GetTickFPS))) 3.6 0.01)))
  (Variables|Hidden|SetLastCourseDistance (Variables|Hidden|GetCourseDistance)))

(fn SingleWheelVibration
  (params (Wheel%20Mesh :type Scene%20Component%20Object%20Reference) (Offset :type Float%20%28double-precision%29))
  (bind _returnvalue (Transformation|GetWorldLocation Wheel%20Mesh))
  ;[0 1 1] Apply Vibration to Each Wheel
  (Transformation|SetWorldLocation Wheel%20Mesh (Math|Vector|MakeVector (.x _returnvalue) (.y _returnvalue) (+ (.z _returnvalue) (Utilities|WheelVibration Offset))) false false))

(fn Vibrations
  (bind _bodyvibrationamount (Variables|Vibrations|GetBodyVibrationAmount))
  (bind _bodyvibrationspeed (Variables|Vibrations|GetBodyVibrationSpeed))
  (bind _overallvibrationmultiplier (Variables|Vibrations|GetOverallVibrationMultiplier))
  (bind _returnvalue (Utilities|PerlinNoise 0.0 _bodyvibrationspeed _bodyvibrationamount _overallvibrationmultiplier))
  ;[0 1 1] Apply Vibration to All Wheels
  (CallFunction|SingleWheelVibration (Variables|Default|GetWheel%20RR) 0.0)
  (CallFunction|SingleWheelVibration (Variables|Default|GetWheel%20RL) 1.0)
  (CallFunction|SingleWheelVibration (Variables|Default|GetWheel%20FR) 2.0)
  (CallFunction|SingleWheelVibration (Variables|Default|GetWheel%20FL) 3.0)
  ;[0 1 0] Apply Vibration to Body
  (Transformation|SetRelativeLocationAndRotation (Variables|Default|GetBody) (Math|Vector|MakeVector 0.0 0.0 (+ (Variables|CarSetup|GetBodyHeight) _returnvalue (Math|Float|MapRangeClamped (Variables|Suspension|GetSuspensionStiffness) 0.0 1e+01 0.0 5.0))) (Math|Rotator|MakeRotator (Variables|Suspension|GetBodyRoll) (+ (Variables|Suspension|GetBodyPitch) (/ _returnvalue 1.5)) 0.0) false false))

(fn CarMeshSetup
  (bind _rearwheelsmesh (Variables|CarSetup|GetRearWheelsMesh))
  (bind _frontcalipersmesh (Variables|CarSetup|GetFrontCalipersMesh))
  (bind _rearcalipersmesh (Variables|CarSetup|GetRearCalipersMesh))
  (bind _frontwheelsmesh (Variables|CarSetup|GetFrontWheelsMesh))
  ;[0 1 0] Set Body Mesh
  (Components|StaticMesh|SetStaticMesh (Variables|Default|GetBody) (Variables|CarSetup|GetBodyMesh))
  ;[0 1 1] Set Wheel Meshes
  (Components|StaticMesh|SetStaticMesh (Variables|Default|GetWheel%20FR) _frontwheelsmesh)
  (Components|StaticMesh|SetStaticMesh (Variables|Default|GetWheel%20FL) _frontwheelsmesh)
  (Components|StaticMesh|SetStaticMesh (Variables|Default|GetWheel%20RR) _rearwheelsmesh)
  (Components|StaticMesh|SetStaticMesh (Variables|Default|GetWheel%20RL) _rearwheelsmesh)
  ;[1 1 0] Set Caliper Meshes
  (Components|StaticMesh|SetStaticMesh (Variables|Default|GetCaliper%20FR) _frontcalipersmesh)
  (Components|StaticMesh|SetStaticMesh (Variables|Default|GetCaliper%20FL) _frontcalipersmesh)
  (Components|StaticMesh|SetStaticMesh (Variables|Default|GetCaliper%20RR) _rearcalipersmesh)
  (Components|StaticMesh|SetStaticMesh (Variables|Default|GetCaliper%20RL) _rearcalipersmesh))

(fn CalculateDistance
  (bind _path (Variables|Driving|GetPath))
  (bind _distancetraveled (Variables|Driving|GetDistanceTraveled))
  (bind _spline (Variables|/RatSim/CinematicCarRig/Blueprints/BP_Path.BP_Path_C|GetSpline _path))
  (bind _returnvalue (Spline|GetSplineLength _spline))
  ;[1 0 0] Calculate the Real Distance from Start when the Distance is Greater than Spline Length
  (Utilities|IsValid (Variables|Driving|GetPath)
    (:Is%20Valid
      (Variables|Hidden|SetLaps (Math|Conversions|ToFloat(Integer) (.ReturnValue (Math|Float|Division(WholeandRemainder) (Variables|Driving|GetDistanceTraveled) _returnvalue))))
      (Variables|Hidden|SetCourseDistance (- _distancetraveled (* _returnvalue (Variables|Hidden|GetLaps)))))
    (:Is%20Not%20Valid
      (Variables|Hidden|SetCourseDistance _distancetraveled))))

(fn ChassisRollandPitch
  (bind _wheel_fl (Variables|Default|GetWheel%20FL))
  (bind _wheel_rl (Variables|Default|GetWheel%20RL))
  (bind _wheel_rr (Variables|Default|GetWheel%20RR))
  (bind _rearaxleoffset (Variables|CarSetup|GetRearAxleOffset))
  (bind _frontaxleoffset (Variables|CarSetup|GetFrontAxleOffset))
  (bind _frontwheelssideoffset (Variables|CarSetup|GetFrontWheelsSideOffset))
  (bind _wheel_fr (Variables|Default|GetWheel%20FR))
  (bind _array (Utilities|Array|MakeArray _wheel_fl _wheel_fr _wheel_rl _wheel_rr))
  (bind _returnvalue (* _frontwheelssideoffset 2.0))
  (bind _returnvalue_2 (+ _rearaxleoffset _frontaxleoffset))
  (bind _output (Utilities|Array|Get(acopy) _array 3))
  (bind _output_2 (Utilities|Array|Get(acopy) _array 2))
  (bind _output_3 (Utilities|Array|Get(acopy) _array))
  (bind _output_4 (Utilities|Array|Get(acopy) _array 1))
  (bind _returnvalue_3 (Transformation|GetWorldLocation _output_2))
  (bind _returnvalue_4 (Transformation|GetWorldLocation _output_3))
  (bind _returnvalue_5 (Transformation|GetWorldLocation _output_4))
  (bind _returnvalue_6 (Transformation|GetWorldLocation _output))
  ;[1 0 0] Calculate Chassis Roll Based on Wheels Location
  (Variables|Hidden|SetChassisRoll (Math|Float|Clamp(Float) (/ (+ (Class|KismetMathLibrary|DegAsin (/ (- (.z _returnvalue_4) (.z _returnvalue_5)) _returnvalue)) (Class|KismetMathLibrary|DegAsin (/ (- (.z _returnvalue_3) (.z _returnvalue_6)) _returnvalue))) 2.0) -85.0 85.0))
  ;[1 0 0] Calculate Chassis Pitch Based on Wheels Location
  (Variables|Hidden|SetChassisPitch (Math|Float|Clamp(Float) (/ (+ (Class|KismetMathLibrary|DegAsin (/ (- (.z _returnvalue_4) (.z _returnvalue_3)) _returnvalue_2)) (Class|KismetMathLibrary|DegAsin (/ (- (.z _returnvalue_5) (.z _returnvalue_6)) _returnvalue_2))) 2.0) -85.0 85.0)))

(fn ChassisRelocation
  (bind _returnvalue (Transformation|GetActorTransform))
  (bind _wheel_rr (Variables|Default|GetWheel%20RR))
  (bind _wheel_rl (Variables|Default|GetWheel%20RL))
  (bind _wheel_fr (Variables|Default|GetWheel%20FR))
  (bind _wheel_fl (Variables|Default|GetWheel%20FL))
  (bind _array (Utilities|Array|MakeArray _wheel_fl _wheel_fr _wheel_rl _wheel_rr))
  (bind _output (Utilities|Array|Get(acopy) _array 3))
  (bind _output_2 (Utilities|Array|Get(acopy) _array 2))
  (bind _output_3 (Utilities|Array|Get(acopy) _array))
  (bind _output_4 (Utilities|Array|Get(acopy) _array 1))
  (bind _returnvalue_2 (Transformation|GetWorldLocation _output))
  (bind _returnvalue_3 (Transformation|GetWorldLocation _output_3))
  (bind _returnvalue_4 (Transformation|GetWorldLocation _output_4))
  (bind _returnvalue_5 (Transformation|GetWorldLocation _output_2))
  (bind _array_2 (Utilities|Array|MakeArray _returnvalue_3 _returnvalue_4 _returnvalue_5 _returnvalue_2))
  (bind _returnvalue_6 (Math|Vector|GetVectorArrayAverage _array_2))
  (bind _returnvalue_7 (Math|Transform|InverseTransformLocation _returnvalue _returnvalue_6))
  ;[1 0 0] Relocate Chassis to the Average of Wheel Locations
  (Transformation|SetRelativeLocation (Variables|Default|GetChassis) (Math|Vector|MakeVector (- (.x _returnvalue_7) (/ (- (Variables|CarSetup|GetFrontAxleOffset) (Variables|CarSetup|GetRearAxleOffset)) 2.0)) (.y _returnvalue_7) (.z _returnvalue_7)) false false))

(fn ActorGroundTrace
  (bind _returnvalue (Transformation|GetActorLocation))
  (bind _returnvalue_2 (Transformation|GetActorLocation))
  (Transformation|SetActorScale3D "1.000000,1.000000,1.000000")
  (if (Variables|CarSetup|GetTraceGround)
    ;[0 0 1] Relocate Actor on the Ground
    (bind _outhit (Collision|LineTraceByChannel (Math|Vector|MakeVector (.x _returnvalue) (.y _returnvalue) (+ (.z _returnvalue) 1.5e+02)) (Math|Vector|MakeVector (.x _returnvalue) (.y _returnvalue) (+ (.z _returnvalue) -1e+04)) "TraceTypeQuery1" true (Variables|Hidden|GetActorsToIgnore) (Variables|CarSetup|GetTraceDebug)))
    (if (.bblockinghit _outhit)
      (Transformation|SetActorLocationAndRotation (.impactpoint _outhit) (Math|Rotator|MakeRotator 0.0 0.0 (.yaw (Transformation|GetActorRotation))))
      (else
        ;[0 0 1] Trace Higher if the Previous one Failed
        (bind _outhit_2 (Collision|LineTraceByChannel (Math|Vector|MakeVector (.x _returnvalue_2) (.y _returnvalue_2) (+ (.z _returnvalue_2) 1e+04)) (Math|Vector|MakeVector (.x _returnvalue_2) (.y _returnvalue_2) (+ (.z _returnvalue_2) -1e+04)) "TraceTypeQuery1" true (Variables|Hidden|GetActorsToIgnore) (Variables|CarSetup|GetTraceDebug)))
        (if (.bblockinghit _outhit_2)
          (Transformation|SetActorLocationAndRotation (.impactpoint _outhit_2) (Math|Rotator|MakeRotator 0.0 0.0 (.yaw (Transformation|GetActorRotation))))
          (else
            ;[1 0 1] Set Default Chassis Values When Not Traced
            (Variables|Hidden|SetChassisRoll 0.0 :!label _label)
            (Variables|Hidden|SetChassisPitch 0.0)))))
    (else
      (goto _label))))

(fn BodyDelay
  (params (Delay :type Boolean))
  (bind _chassis (Variables|Default|GetChassis))
  (bind _suspensionstiffness (Variables|Suspension|GetSuspensionStiffness))
  (bind _body_and_accessories (Variables|Default|GetBody%20and%20Accessories))
  (bind _tickfps (Variables|CarSetup|GetTickFPS))
  (bind _chassis_2 (Variables|Default|GetChassis))
  (bind _returnvalue (Transformation|GetWorldRotation _body_and_accessories))
  (bind _returnvalue_2 (Transformation|GetWorldRotation _chassis))
  (bind _returnvalue_3 (Transformation|GetWorldTransform _chassis))
  (bind _returnvalue_4 (Math|Float|MapRangeClamped _suspensionstiffness 0.0 1e+01 3.0 15.0))
  (bind _returnvalue_5 (/ 1.0 _tickfps))
  (bind _returnvalue_6 (Math|Interpolation|RInterpTo _returnvalue _returnvalue_2 _returnvalue_5 _returnvalue_4))
  (if Delay
    ;[0 1 0] Body Transform Delay for Z Location, Roll and Pitch
    (Transformation|SetWorldLocationAndRotation (Variables|Default|GetBody%20and%20Accessories) (Math|Transform|TransformLocation _returnvalue_3 (Math|Vector|MakeVector 0.0 0.0 (Math|Interpolation|FInterpTo (.z (Math|Transform|InverseTransformLocation _returnvalue_3 (Transformation|GetWorldLocation _body_and_accessories))) 0.0 _returnvalue_5 _returnvalue_4))) (Math|Rotator|MakeRotator (.roll _returnvalue_6) (.pitch _returnvalue_6) (.yaw (Transformation|GetWorldRotation _chassis))) false false)
    (else
      ;[0 1 0] To Prevent Body Delay in Construction Script
      (Transformation|SetWorldLocationAndRotation (Variables|Default|GetBody%20and%20Accessories) (Transformation|GetWorldLocation _chassis_2) (Transformation|GetWorldRotation _chassis_2) false false))))

(fn SetTraceIgnores
  ;[1 0 0] Get All the Actors to Ignore in Trace
  (bind _outactors (Actor|GetAllActorswithTag "IgnoreTrace"))
  (Variables|Hidden|SetActorsToIgnore _outactors))

(fn StartEditorTick
  (if (Variables|CarSetup|GetEditorUpdate)
    (Utilities|Time|SetTimerbyFunctionName 0 "EditorTick" (/ 1.0 (Variables|CarSetup|GetTickFPS)) true)))

(fn AutoMove
  (params (DeltaSec :type Float%20%28double-precision%29))
  (if (Variables|Driving|GetIfAutoMove)
    (Variables|Driving|SetDistanceTraveled (+ (* DeltaSec 1e+02) (Variables|Driving|GetDistanceTraveled)))))