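; BP_Husky is a Husky pawn Blueprint that extends its parent with trajectory display and lidar visualization.
; The construction script hands the Path spline to the TrajectoryViewer.
; BeginPlay caches the viewer's last traveled distance as an offset, and Tick adds it to DistanceTraveled to drive the viewer's progress.
; Vis4Lidar triggers point cloud visualization on the LidarC component.
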(event EventEditorTick
  (|CallParentFunction))

(event EventTick
  (params (DeltaSeconds :type Float%20%28single-precision%29))
  (|CallParentFunction DeltaSeconds)
  (Variables|/Script/RatSim.TrajectoryViewer|SetTraveledDistance (Variables|Default|GetTrajectoryViewer) (+ (Variables|Default|GetDistanceTraveled) (Variables|Default|GetStartOffset))))

(event EventBeginPlay
  (|CallParentFunction)
  (Variables|Default|SetStartOffset (Variables|/Script/RatSim.TrajectoryViewer|GetLastTraveledDistance (Variables|Default|GetTrajectoryViewer))))

(fn ConstructionScript
  (|CallParentFunction)
  (Variables|/Script/RatSim.TrajectoryViewer|SetSplineComponent (Variables|Default|GetTrajectoryViewer) (Variables|/RatSim/CinematicCarRig/Blueprints/BP_Path.BP_Path_C|GetSpline (Variables|Default|GetPath))))

(fn Vis4Lidar
  (Class|LidarComponent|VisualizePointCloud (Variables|Default|GetLidarC)))